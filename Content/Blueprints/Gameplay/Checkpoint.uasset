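; Checkpoint actor that swaps the player's pawn for a different pawn class on overlap.
; When the overlapping actor's class exactly matches SourcePawnClass, it plays an explosion effect and destroys that actor.
; It then spawns TargetPawnClass at the saved transform and has player controller 0 possess the new pawn.
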(event `self.ReceiveActorBeginOverlap`
  (params (OtherActor :type "Actor Object Reference"))
  (bind (_actortransform_location _actortransform_rotation) (`KismetMathLibrary.BreakTransform` (`self.ActorTransform`)))
  (set `self.SourcePawn` OtherActor)
  (set `self.ActorTransform` (`self.GetTransform` (`self.SourcePawn`)))
  (if (== (`GameplayStatics.GetObjectClass` (`self.SourcePawn`)) (`self.SourcePawnClass`))
    (`GameplayStatics.SpawnEmitterAtLocation` "/Game/CartoonFX2/Particles/PS_Explosion.PS_Explosion" _actortransform_location _actortransform_rotation)
    (`self.K2_DestroyActor` (`self.SourcePawn`))
    (bind _returnvalue (`|SpawnActorFromClass` (`self.TargetPawnClass`) (`self.ActorTransform`) (`self.CollisionHandlingOverride`) "OverrideRootScale" null null))
    (`Controller.Possess` (`GameplayStatics.GetPlayerController` 0) _returnvalue)))

(fn `UserConstructionScript`)